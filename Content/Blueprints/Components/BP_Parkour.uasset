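; Parkour component that gives a character wallrunning, wall jumps and detaching.
; After Init, a looping timer traces right and left for near-vertical walls, launching the falling character along the normal's cross product and easing gravity toward a target.
; Jumping or detaching launches it off the wall normal, while resets restore gravity and briefly suppress wallrunning.
; Tick rolls the camera by wall side, and wallrun start and reset drive BP_Character's sprint camera animation.
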(event Custom|Init
  (params (Character :type Player%20Chr%20Object%20Reference))
  (bind _output_get (Variables|Default|SetCharacter Character))
  (bind _output_get_2 (Variables|Default|SetCharacter%20Movement (Variables|/Script/Engine.Character|GetCharacterMovement _output_get)))
  (Variables|Default|SetDefaultGravity (Variables|/Script/Engine.CharacterMovementComponent|GetGravityScale _output_get_2))
  (Utilities|Time|SetTimerbyEvent (delegate Custom|WRE_Update) 0.02 true))

(event Custom|WRE_Update
  (if (not (Variables|Default|GetbWR_Suppressed))
    (CallFunction|WRUpdate)))

(event Custom|OnJump
  (CallFunction|WRJump))

(event Custom|WR_ResetSuppression
  (Utilities|Time|ClearTimerbyFunctionName self "WR_ResetSuppression")
  (Variables|Default|SetbWR_Suppressed false))

(event Custom|OnLanding
  (CallFunction|WRReset 0.0)
  (Variables|Default|SetbWR_Suppressed false))

(event EventTick
  (params (DeltaSeconds :type Float%20%28single-precision%29))
  (CallFunction|CameraTick))

(fn WRMovement
  (params (Start :type Vector) (End :type Vector) (Direction :type Float%20%28single-precision%29))
  (bind _outhit (Collision|LineTraceByChannel Start End "TraceTypeQuery1" false 0 "None"))
  (if (.bblockinghit _outhit)
    (Variables|Default|SetWR_Normal (.OutVec (Utilities|IsValidVector? (.normal _outhit))))
    (if (and (AI|Components|NavMovement|IsFalling (Variables|Default|GetCharacter%20Movement)) (.ReturnValue (Utilities|IsValidVector? (.normal _outhit))))
      (Character|LaunchCharacter (Variables|Default|GetCharacter) (* (Math|Vector|CrossProduct (Variables|Default|GetWR_Normal) "0, 0,2.000000") (* (Variables|Default|GetWR_Speed) Direction)) true (not (Variables|Default|GetbWR_Gravity)))
      (return true)
      (else
        (return false)))
    (else
      (return false))))

(fn WRReset
  (params (ResetTime :type Float%20%28single-precision%29))
  (if (Variables|/Script/aleph.PlayerChr|GetbIsWallrunning (Variables|Default|GetCharacter))
    (bind _output_get (Variables|/Script/aleph.PlayerChr|SetbIsWallrunning (Variables|Default|GetCharacter) false))
    (bind _output_get_2 (Variables|Default|SetbWR_Left _output_get))
    (Variables|Default|SetbWR_Right _output_get_2)
    (Variables|/Script/Engine.CharacterMovementComponent|SetGravityScale (Variables|Default|GetCharacter%20Movement) (Variables|Default|GetDefaultGravity))
    (CallFunction|WRSuppress ResetTime)
    (bind _asbp_character (Utilities|Casting|CastToBP_Character (Variables|Default|GetCharacter)))
    (Default|AnimReverseSprintCamera _asbp_character)))

(fn WRSuppress
  (params (Delay :type Float%20%28single-precision%29))
  (Variables|Default|SetbWR_Suppressed true)
  (Utilities|Time|SetTimerbyFunctionName self "WR_ResetSuppression" Delay))

(fn WRJump
  (bind _wr_normal (Variables|Default|GetWR_Normal))
  (if (Variables|/Script/aleph.PlayerChr|GetbIsWallrunning (Variables|Default|GetCharacter))
    (CallFunction|WRReset 0.25)
    (Character|LaunchCharacter (Variables|Default|GetCharacter) (Math|Vector|MakeVector (* (Variables|Default|GetWR_JumpForce) (.x _wr_normal)) (* (Variables|Default|GetWR_JumpForce) (.y _wr_normal)) (Variables|Default|GetWR_JumpForce)) false true)))

(fn WRUpdate
  (bind _onwall (CallFunction|WRMovement (Transformation|GetActorLocation (Variables|Default|GetCharacter)) (.Right (Utilities|EndVectors)) -1.0))
  (if _onwall
    (bind _output_get (Variables|/Script/aleph.PlayerChr|SetbIsWallrunning (Variables|Default|GetCharacter) true))
    (Variables|Default|SetbWR_Right _output_get)
    (Variables|Default|SetbWR_Left false)
    (Variables|/Script/Engine.CharacterMovementComponent|SetGravityScale (Variables|Default|GetCharacter%20Movement) (Utilities|GravMacro) :!label _label)
    (bind _asbp_character (Utilities|Casting|CastToBP_Character (Variables|Default|GetCharacter)))
    (Default|AnimSprintCamera _asbp_character 95.0)
    (elif (Variables|Default|GetbWR_Right)
      (CallFunction|WRReset 0.25)
      (else
        (bind _onwall_2 (CallFunction|WRMovement (Transformation|GetActorLocation (Variables|Default|GetCharacter)) (.Left (Utilities|EndVectors)) 1.0))
        (if _onwall_2
          (bind _output_get_2 (Variables|/Script/aleph.PlayerChr|SetbIsWallrunning (Variables|Default|GetCharacter) true))
          (Variables|Default|SetbWR_Left _output_get_2)
          (Variables|Default|SetbWR_Right false)
          (goto _label)
          (else
            (CallFunction|WRReset 0.25)))))))

(fn WRDetach
  (params (ResetTime :type Float%20%28single-precision%29))
  (bind _wr_normal (Variables|Default|GetWR_Normal))
  (if (Variables|/Script/aleph.PlayerChr|GetbIsWallrunning (Variables|Default|GetCharacter))
    (CallFunction|WRReset ResetTime)
    (Character|LaunchCharacter (Variables|Default|GetCharacter) (Math|Vector|MakeVector (* (Variables|Default|GetWR_JumpForce) (.x _wr_normal)) (* (Variables|Default|GetWR_JumpForce) (.y _wr_normal)) 15.0) false true)))

(fn CameraTick
  (if (Variables|Default|GetbWR_Left)
    (CallFunction|CameraTilt 15.0)
    (elif (Variables|Default|GetbWR_Right)
      (CallFunction|CameraTilt -15.0)
      (else
        (CallFunction|CameraTilt 0.0)))))

(fn CameraTilt
  (params (X%20%28Roll%29 :type Float%20%28single-precision%29))
  (bind _character (Variables|Default|GetCharacter))
  (bind _returnvalue (Pawn|GetController _character))
  (bind _returnvalue_2 (Pawn|GetControlRotation _returnvalue :!class /Script/Engine.Controller))
  (bind (_roll _pitch _yaw) (Math|Rotator|BreakRotator _returnvalue_2))
  (Pawn|SetControlRotation (Pawn|GetController (Variables|Default|GetCharacter)) (Math|Interpolation|RInterpTo _returnvalue_2 (Math|Rotator|MakeRotator X%20%28Roll%29 _pitch _yaw) (Utilities|Time|GetWorldDeltaSeconds) 1e+01)))