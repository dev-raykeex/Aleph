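; BP_Instance, apparently the game instance for the Aleph project, posts a startup report to the in-game console.
; On Init it sends short, delayed messages with the build version, current level, CPU, memory, GPU and current GameType.
; AddMessageToConsole relays each message to every widget implementing BPI_conSole, so senders need no direct widget reference.
; GiveBasicInfo is an empty stub.
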(event EventInit
  (Utilities|FlowControl|Delay 0.2)
  (bind _returnvalue (Game|GetCurrentLevelName true))
  (CallFunction|AddMessagetoConsole "aleph" "Warning" (Utilities|Text|FormatText "Welcome to Aleph-UE5-0.4-Alpha. | Current level: {LevelName}." _returnvalue))
  (Utilities|FlowControl|Delay 0.2)
  (CallFunction|AddMessagetoConsole "aleph" "Notice" (Utilities|Text|FormatText "CPU: {Brand} ({Cores} cores/{Threads} threads) " (Class|HardwareDetails|GetCPUBrand) (Class|HardwareDetails|GetCPUCores) (Class|HardwareDetails|GetCPUThreads)))
  (Utilities|FlowControl|Delay 0.2)
  (CallFunction|AddMessagetoConsole "aleph" "Notice" (Utilities|Text|FormatText "Memory: {Capacity} GB" (Class|HardwareDetails|GetRAMCapacity)))
  (Utilities|FlowControl|Delay 0.2)
  (CallFunction|AddMessagetoConsole "aleph" "Notice" (Utilities|Text|FormatText "GPU: {Brand}" (Class|HardwareDetails|GetGPUBrand)))
  (Utilities|FlowControl|Delay 0.2)
  (CallFunction|AddMessagetoConsole "aleph" "Warning" (Utilities|Text|FormatText "The GameType is currently set on: {GameType}." (Variables|Default|GetGameType))))

(fn AddMessagetoConsole
  (params (Component :type String) (Code :type String) (Message :type Text))
  (bind _foundwidgets (Class|WidgetBlueprintLibrary|GetAllWidgetswithInterface "/conSole/Blueprints/BPI_conSole.BPI_conSole_C" false))
  (for _array_element _foundwidgets
    (Class|BPIConSole|AddMessagetoConsole(Message) _array_element Component Code Message)))

(fn GiveBasicInfo)