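; Enemy drone AI that detects the player character, notifies them and attacks.
; On sighting, it records the player's location, fires an impulse-driven projectile with a delay-based cooldown, and moves to that location.
; A DoOnce limits detection alerts until that move succeeds.
; It picks a random reachable idle point at BeginPlay, but the timeline logic for wandering there is unconnected and never runs.
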(event OnSeePawn(PawnSensing)
  (params (Pawn :type Pawn%20Object%20Reference))
  (bind _asbp_character (Utilities|Casting|CastToBP_Character Pawn))
  (Utilities|FlowControl|Sequence
    (:then_0
      (Variables|Default|SetLastKnownLocation (Transformation|GetActorLocation _asbp_character))
      (Utilities|FlowControl|DoOnce false :!label _label
        (:Completed
          (Default|SendNotification _asbp_character "You've been detected" "(R=0.102500,G=0.150000,B=0.000000,A=0.700000)" true 3.5))))
    (:then_1
      (if (Variables|Default|GetSpawnProjectile)
        (Variables|Default|SetInCombat true)
        (bind _returnvalue (Game|SpawnActorfromClass "/Game/Imported/FirstPersonProjectile.FirstPersonProjectile_C" (Transformation|GetWorldTransform (Variables|Default|GetBulletSpawnLocation)) "Undefined" 0 0))
        (Physics|AddImpulse (Variables|/Game/Imported/FirstPersonProjectile.FirstPersonProjectile_C|GetSphere _returnvalue) (* (Math|Vector|GetForwardVector (Variables|Default|GetSphere)) (Variables|Default|GetShootAmount)) "None" true)
        (Variables|Default|SetSpawnProjectile false)
        (Utilities|FlowControl|Delay 1e+01)
        (Variables|Default|SetSpawnProjectile true)
        (Variables|Default|SetInCombat false)))
    (:then_2
      (AI|AIMoveTo self (Variables|Default|GetLastKnownLocation) 0 5.0 false
        (:OnSuccess
          (goto _label Reset))))))

(event EventBeginPlay
  (CallFunction|GeneratePathLocation))

(fn ConstructionScript)

(fn GetRandomLocation
  (bind _output_get (Variables|IdlePathLocs|SetCurrentPathPoint (Math|Random|RandomInteger (Utilities|Array|Length (Variables|IdlePathLocs|GetIdlePathArray)))))
  (CallFunction|SendNotification (Utilities|Text|FormatText "{CURRENT_PATH_INDEX}" _output_get) "(R=0.150000,G=0.000000,B=0.000000,A=1.000000)"))

(fn SendNotification
  (params (NotificationToShow :type Text) (NotificationColor :type Linear%20Color%20Structure :default "(R=0.150000,G=0.000000,B=0.000000,A=1.000000)"))
  (Default|AddNotification (Variables|/Game/Blueprints/BP_Instance.BP_Instance_C|GetHeadsUpDisplay (.AsBP%20Instance (Utilities|Casting|CastToBP_Instance (Game|GetGameInstance)))) NotificationToShow NotificationColor true 3.5))

(fn GeneratePathLocation
  (bind _returnvalue (Transformation|GetActorLocation))
  (bind _randomlocation (AI|Navigation|GetRandomReachablePointinRadius _returnvalue 1.5e+03 0 0))
  (Variables|Default|SetIdlePathLocation (Math|Vector|MakeVector (.x _randomlocation) (.y _randomlocation) 1.2e+02))
  (return))