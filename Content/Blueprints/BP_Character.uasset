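; Player character Blueprint handling movement, sensitivity-scaled look, FOV zoom, jumping via a parkour component, and physics-object grabbing.
; Crouch uses a timeline to resize the capsule, with an overhead trace before standing.
; Holding Dash sprints; double-tapping launches directionally, gated and drained by the energy component.
; Tick handles death, health capping, parkour Init, traced custom-depth outlines and debug speed printing; slide logic is unfinished and uncalled.
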(event Custom|UnCrouch%20Event
  (bind _capsulecomponent (Variables|Default|GetCapsuleComponent))
  (bind _returnvalue (Transformation|GetWorldLocation _capsulecomponent))
  ;[1 1 1] Here we'll keep the custom events for the game that we'll use when the Functions can't help us.
  (bind _returnvalue_2 (Collision|SphereTraceByChannel (+ _returnvalue "0, 0,30.000000") (+ _returnvalue "0, 0,90.000000") 45.0 "TraceTypeQuery1" true 0 "Persistent"))
  (if (not _returnvalue_2)
    (Variables|Default|SetIsCrouching false)
    (Variables|/Script/Engine.CharacterMovementComponent|SetMaxWalkSpeed (Variables|Character|GetCharacterMovement) (Variables|Default|GetBaseWalkSpeed))
    (bind _alpha (Timeline|A_Crouch Reverse)
      (:Update
        (Components|Capsule|SetCapsuleHalfHeight (Variables|Default|GetCapsuleComponent) (Math|Float|Lerp 88.0 44.0 _alpha) true)))))

(event Custom|Crouch%20Event
  ;[1 1 1] Here we'll keep the custom events for the game that we'll use when the Functions can't help us.
  (Variables|Default|SetIsCrouching true)
  (Variables|/Script/Engine.CharacterMovementComponent|SetMaxWalkSpeed (Variables|Character|GetCharacterMovement) (Variables|Default|GetBaseCrouchSpeed))
  (bind _alpha (Timeline|A_Crouch Play)
    (:Update
      (Components|Capsule|SetCapsuleHalfHeight (Variables|Default|GetCapsuleComponent) (Math|Float|Lerp 88.0 44.0 _alpha) true))))

(event EventTick
  (params (DeltaSeconds :type Float%20%28single-precision%29))
  ;[1 1 1] This code checks for changes in stats and updates.
  (Utilities|FlowControl|Sequence
    (:then_0
      (CallFunction|FDeath))
    (:then_1
      (CallFunction|FMaxHealthLimit))
    (:then_2
      (Default|Init (Variables|Default|GetParkourComp) self))
    (:then_3
      (CallFunction|FOutline))
    (:then_4
      (Development|PrintString (Utilities|String|ToString(Float) (Variables|/Script/Engine.CharacterMovementComponent|GetMaxWalkSpeed (Variables|Character|GetCharacterMovement)))))))

(event EventOnLanded
  (params (Hit :type Hit%20Result%20Structure%20%28by%20ref%29))
  ;[1 1 1] This is where more advanced movement code will go.
  (Default|EventLand (Variables|Default|GetParkourComp)))

(event Input|ActionEvents|InputActionJump
  (params (Key :type Key%20Structure :default "None"))
  ;[1 1 1] This is where more advanced movement code will go.
  (:Pressed
    (Character|Jump)
    (Default|EventJump (Variables|Default|GetParkourComp)))
  (:Released
    (Character|StopJumping)))

(event Input|ActionEvents|InputActionCrouch
  (params (Key :type Key%20Structure :default "None"))
  ;[1 1 1] This is where more advanced movement code will go.
  (:Pressed
    (if (Variables|Default|GetIsCrouching)
      (CallFunction|UnCrouchEvent)
      (else
        (CallFunction|CrouchEvent)))))

(event Input|ActionEvents|InputActionShowMouse
  (params (Key :type Key%20Structure :default "None"))
  (bind _returnvalue (Game|GetPlayerController 0))
  ;[1 1 1] This is some basic code for the Mouse to appear on Screen while in-game.
  (:Pressed
    (Variables|/Script/Engine.PlayerController|SetbShowMouseCursor _returnvalue true))
  (:Released
    (Variables|/Script/Engine.PlayerController|SetbShowMouseCursor _returnvalue false)))

(event Input|ActionEvents|InputActionZoom
  (params (Key :type Key%20Structure :default "None"))
  ;[1 1 1] This is the Zoom code.
  (:Pressed
    (if (Variables|Default|GetIsZoomed)
      (bind _zoom (Timeline|AZoom Reverse)
        (:Update
          (Camera|SetFieldOfView (Variables|Default|GetCamera) _zoom)
          (Utilities|FlowControl|FlipFlop
            (:A
              (Variables|Default|SetIsZoomed true))
            (:B
              (Variables|Default|SetIsZoomed false)))))
      (else
        (Timeline|AZoom Play)))))

(event Input|ActionEvents|InputActionInteract
  (params (Key :type Key%20Structure :default "None"))
  ;[1 1 1] Interacting code
  (:Pressed
    (bind _hitcomponent (CallFunction|FGrab))
    (Variables|Default|SetHold%20Component _hitcomponent))
  (:Released
    (CallFunction|FGrabStop (Variables|Default|GetPhysicsHandle) (Variables|Default|GetHold%20Component))))

(event Input|ActionEvents|InputActionDash
  (params (Key :type Key%20Structure :default "None"))
  ;[1 1 1] This is where more advanced movement code will go.
  (:Pressed
    (bind _result (Math|Integer|IncrementInt (Variables|Default|GetInputAmount))
      (:%20%20
        (bind _output_get (Variables|Default|SetInputAmount (Math|Integer|Clamp(Integer) _result 0 2)))
        (if (== _output_get 2)
          (bind _returnvalue (CallFunction|FEnergyCheck))
          (if _returnvalue
            (CallFunction|FDash (Input|AxisValues|Getmovement_forward) (Input|AxisValues|Getmovement_side))
            (Variables|Default|SetInputAmount 0)
            (else
              (Utilities|FlowControl|RetriggerableDelay 0.5 :!label _label)
              (Variables|Default|SetInputAmount 0)))
          (elif (not (Variables|Default|GetIsCrouching))
            (Variables|/Script/Engine.CharacterMovementComponent|SetMaxWalkSpeed (Variables|Character|GetCharacterMovement) (* (Variables|Default|GetBaseWalkSpeed) (Variables|Default|GetBaseWalkMultiplier)))
            (goto _label))))))
  (:Released
    (if (> (Variables|/Script/Engine.CharacterMovementComponent|GetMaxWalkSpeed (Variables|Character|GetCharacterMovement)) (Variables|Default|GetBaseWalkSpeed))
      (Variables|/Script/Engine.CharacterMovementComponent|SetMaxWalkSpeed (Variables|Character|GetCharacterMovement) (Variables|Default|GetBaseWalkSpeed)))))

(event Input|AxisEvents|InputAxislook_horizontal
  (params (AxisValue :type Float%20%28single-precision%29))
  ;[1 1 1] This is some mouse movement code.
  (CallFunction|FHorizontalLook AxisValue)
  (CallFunction|FGrabLocation))

(event Input|AxisEvents|InputAxislook_vertical
  (params (AxisValue :type Float%20%28single-precision%29))
  ;[1 1 1] This is some mouse movement code.
  (CallFunction|FVerticalLook AxisValue)
  (CallFunction|FGrabLocation))

(event Input|AxisEvents|InputAxismovement_forward
  (params (AxisValue :type Float%20%28single-precision%29))
  ;[1 1 1] Some basic character movement code.
  (Variables|Default|SetIsWalkingV true)
  (CallFunction|FForwardMovement AxisValue)
  (if (== AxisValue 0.0)
    (Utilities|FlowControl|RetriggerableDelay 0.5)
    (Variables|Default|SetIsWalkingV false)))

(event Input|AxisEvents|InputAxismovement_side
  (params (AxisValue :type Float%20%28single-precision%29))
  ;[1 1 1] Some basic character movement code.
  (Variables|Default|SetIsWalkingH true)
  (CallFunction|FSideMovement AxisValue)
  (if (== AxisValue 0.0)
    (Utilities|FlowControl|RetriggerableDelay 0.5)
    (Variables|Default|SetIsWalkingH false)))

(event Input|AxisEvents|InputAxisTurnRate
  (params (AxisValue :type Float%20%28single-precision%29))
  ;[1 1 1] This is some gamepad movement code.
  (CallFunction|FTurnRate AxisValue))

(event Input|AxisEvents|InputAxisLookRate
  (params (AxisValue :type Float%20%28single-precision%29))
  ;[1 1 1] This is some gamepad movement code.
  (CallFunction|FLookRate AxisValue))

(event Input|MouseEvents|MouseWheelUp
  (params (Key :type Key%20Structure :default "None"))
  ;[1 1 1] This is the Zoom code.
  (:Pressed
    (CallFunction|FZoomin)))

(event Input|MouseEvents|MouseWheelDown
  (params (Key :type Key%20Structure :default "None"))
  ;[1 1 1] This is the Zoom code.
  (:Pressed
    (CallFunction|FZoomOut)))

(fn ConstructionScript)

(fn FCrouch
  (params (Condition :type Boolean))
  (if Condition
    (Variables|/Script/Engine.CharacterMovementComponent|SetMaxWalkSpeed (Variables|Character|GetCharacterMovement) (Variables|Default|GetBaseCrouchSpeed))
    (else
      (Variables|/Script/Engine.CharacterMovementComponent|SetMaxWalkSpeed (Variables|Character|GetCharacterMovement) (Variables|Default|GetBaseWalkSpeed)))))

(fn FDash
  (params (AxisV :type Float%20%28single-precision%29) (AxisH :type Float%20%28single-precision%29))
  (bind _returnvalue (Transformation|GetActorRightVector))
  (bind _returnvalue_2 (Transformation|GetActorForwardVector))
  (Utilities|FlowControl|Sequence
    (:then_0
      (if (Variables|Default|GetIsWalkingV)
        (if (== AxisV 1.0)
          (Variables|Default|SetD_Axis 5e+03)
          (if (not (Variables|Default|GetIsCrouching)) :!label _label
            (Character|LaunchCharacter (Math|Vector|MakeVector (* (.x _returnvalue_2) (Variables|Default|GetD_Axis)) (* (.y _returnvalue_2) (Variables|Default|GetD_Axis)) (.z _returnvalue_2)) false false)
            (CallFunction|FRemoveEnergy 15))
          (elif (== AxisV -1.0)
            (Variables|Default|SetD_Axis -5e+03)
            (goto _label)))))
    (:then_1
      (if (Variables|Default|GetIsWalkingH)
        (if (== AxisH 1.0)
          (Variables|Default|SetD_Axis 5e+03)
          (if (not (Variables|Default|GetIsCrouching)) :!label _label_2
            (Character|LaunchCharacter (Math|Vector|MakeVector (* (.x _returnvalue) (Variables|Default|GetD_Axis)) (* (.y _returnvalue) (Variables|Default|GetD_Axis)) (.z _returnvalue)) false false)
            (CallFunction|FRemoveEnergy 15))
          (elif (== AxisH -1.0)
            (Variables|Default|SetD_Axis -5e+03)
            (goto _label_2)))))))

(fn FDashFailed
  (bind _emergycomp (Variables|Default|GetEmergyComp))
  (bind _returnvalue (Class|EPC|GetEnergy _emergycomp))
  (bind _returnvalue_2 (- 50 _returnvalue))
  (bind _result (Utilities|Text|FormatText "You need {EPC_Required} EPC to do this action" _returnvalue_2))
  (if (< _returnvalue 50)
    (bind _returnvalue_3 (UserInterface|CreateWidget "/Game/Widgets/Elements/Notifications/DashNotif.DashNotif_C"))
    (Default|GetDashMessage _returnvalue_3 _result)
    (UserInterface|Viewport|AddtoViewport _returnvalue_3 0)
    (Development|PrintString (Utilities|String|ToString(Text) _result) false)))

(fn FDeath
  (if (<= (Class|HPC|GetHealth (Variables|Default|GetHealthComp)) 0)
    (Actor|DestroyActor)
    (Development|PrintString "YOU DEAD :)" true true "(R=0.000000,G=0.660000,B=1.000000,A=1.000000)" 5.0)))

(fn FEnergyCheck
  (bind _emergycomp (Variables|Default|GetEmergyComp))
  (bind _returnvalue (Class|EPC|GetEnergy _emergycomp))
  (bind _returnvalue_2 (>= _returnvalue 50))
  (if _returnvalue_2
    (return _returnvalue_2)
    (else
      (CallFunction|FDashFailed))))

(fn FForwardMovement
  (params (Axis :type Float%20%28single-precision%29))
  (Pawn|Input|AddMovementInput (Transformation|GetActorForwardVector) Axis false))

(fn FSideMovement
  (params (Axis :type Float%20%28single-precision%29))
  (Pawn|Input|AddMovementInput (Transformation|GetActorRightVector) Axis false))

(fn FGrab
  (bind _camera (Variables|Default|GetCamera))
  (bind _returnvalue (Transformation|GetWorldLocation _camera))
  (bind (_outhit _returnvalue_2) (Collision|LineTraceForObjects _returnvalue (+ (* (Math|Vector|GetForwardVector _camera) 256.0) _returnvalue) (Utilities|Array|MakeArray "ObjectTypeQuery4") false 0 "None"))
  (if _returnvalue_2
    (Class|PhysicsHandleComponent|GrabComponentatLocation (Variables|Default|GetPhysicsHandle) (.HitComponent (Collision|BreakHitResult _outhit)) "None" (Transformation|GetWorldLocation (.HitComponent (Collision|BreakHitResult _outhit))))
    (Class|PrimitiveComponent|SetAngularDamping (.HitComponent (Collision|BreakHitResult _outhit)) 5.0)
    (Variables|Default|SetIsGrabbing true)
    (return (.HitComponent (Collision|BreakHitResult _outhit)))))

(fn FGrabStop
  (params (PhysicsHandle :type Physics%20Handle%20Component%20Object%20Reference) (GrabbedObject :type Primitive%20Component%20Object%20Reference))
  (Utilities|IsValid GrabbedObject
    (:Is%20Valid
      (Physics|Components|PhysicsHandle|ReleaseComponent PhysicsHandle)
      (Class|PrimitiveComponent|SetAngularDamping GrabbedObject 0.0)
      (Variables|Default|SetIsGrabbing false))))

(fn FGrabLocation
  (bind _camera (Variables|Default|GetCamera))
  (Physics|Components|PhysicsHandle|SetTargetLocation (Variables|Default|GetPhysicsHandle) (+ (* (Math|Vector|GetForwardVector _camera) (Variables|Default|GetGrabDistance)) (Transformation|GetWorldLocation _camera))))

(fn FHorizontalLook
  (params (Axis :type Float%20%28single-precision%29))
  (bind _asbp_instance (Utilities|Casting|CastToBP_Instance (Game|GetGameInstance)))
  (Utilities|IsValid _asbp_instance
    (:Is%20Valid
      (Pawn|Input|AddControllerYawInput (* Axis (Class|GInstance|GetMouseSensitivity _asbp_instance))))))

(fn FVerticalLook
  (params (Axis :type Float%20%28single-precision%29))
  (bind _asbp_instance (Utilities|Casting|CastToBP_Instance (Game|GetGameInstance)))
  (Utilities|IsValid _asbp_instance
    (:Is%20Valid
      (Pawn|Input|AddControllerPitchInput (* Axis (Class|GInstance|GetMouseSensitivity _asbp_instance))))))

(fn FZoomin
  (bind _camera (Variables|Default|GetCamera))
  (Utilities|IsValid _camera
    (:Is%20Valid
      (if (not (<= (Variables|/Script/Engine.CameraComponent|GetFieldOfView _camera) 32.0))
        (Variables|/Script/Engine.CameraComponent|SetFieldOfView _camera (- (Variables|/Script/Engine.CameraComponent|GetFieldOfView _camera) 5.0))))))

(fn FZoomOut
  (bind _camera (Variables|Default|GetCamera))
  (Utilities|IsValid _camera
    (:Is%20Valid
      (if (not (>= (Variables|/Script/Engine.CameraComponent|GetFieldOfView _camera) 9e+01))
        (Variables|/Script/Engine.CameraComponent|SetFieldOfView _camera (+ (Variables|/Script/Engine.CameraComponent|GetFieldOfView _camera) 5.0))))))

(fn FTurnRate
  (params (Axis :type Float%20%28single-precision%29))
  (bind _asbp_instance (Utilities|Casting|CastToBP_Instance (Game|GetGameInstance)))
  (Utilities|IsValid _asbp_instance
    (:Is%20Valid
      (Pawn|Input|AddControllerYawInput (* Axis (Class|GInstance|GetGamepadSensitivity _asbp_instance) (Utilities|Time|GetWorldDeltaSeconds))))))

(fn FLookRate
  (params (Axis :type Float%20%28single-precision%29))
  (bind _asbp_instance (Utilities|Casting|CastToBP_Instance (Game|GetGameInstance)))
  (Utilities|IsValid _asbp_instance
    (:Is%20Valid
      (Pawn|Input|AddControllerPitchInput (* Axis (Class|GInstance|GetGamepadSensitivity _asbp_instance) (Utilities|Time|GetWorldDeltaSeconds))))))

(fn FSlideStart
  (bind _charactermovement (Variables|Character|GetCharacterMovement))
  (if (and (Utilities|CanSlide) (Pawn|Components|CharacterMovement|IsWalking (Variables|Character|GetCharacterMovement)))
    (Character|Crouch)
    (Variables|/Script/Engine.CharacterMovementComponent|SetGroundFriction _charactermovement 0.0)
    (Variables|/Script/Engine.CharacterMovementComponent|SetBrakingDecelerationWalking _charactermovement 1.4e+03)
    (Class|MovementComponent|SetPlaneConstraintfromVectors _charactermovement (|V_Normal _charactermovement) (Transformation|GetActorUpVector))
    (Class|MovementComponent|SetPlaneConstraintEnabled _charactermovement true)
    (|GetSlideVector)))

(fn FRemoveEnergy
  (params (Value :type Integer))
  (bind _emergycomp (Variables|Default|GetEmergyComp))
  (Class|EPC|SetEnergy _emergycomp (- (Class|EPC|GetEnergy _emergycomp) Value)))

(fn FMaxHealthLimit
  (bind _healthcomp (Variables|Default|GetHealthComp))
  (Utilities|IsValid _healthcomp
    (:Is%20Valid
      (if (> (Class|HPC|GetHealth _healthcomp) (Variables|/Script/Aleph.HPC|GetDefaultHealth (Variables|Default|GetHealthComp)))
        (Class|HPC|SetHealth _healthcomp 100)))))

(fn FMaxEnergyLimit
  (bind _emergycomp (Variables|Default|GetEmergyComp))
  (Utilities|IsValid _emergycomp
    (:Is%20Valid
      (if (> (Class|EPC|GetEnergy _emergycomp) (Variables|/Script/Aleph.EPC|GetDefaultEnergy (Variables|Default|GetEmergyComp)))
        (Class|EPC|SetEnergy _emergycomp 100)))))

(fn FOutline
  (bind _camera (Variables|Default|GetCamera))
  (bind _returnvalue (Transformation|GetWorldLocation _camera))
  (Utilities|IsValid _camera
    (:Is%20Valid
      (bind (_outhit _returnvalue_2) (Collision|LineTraceForObjects _returnvalue (+ _returnvalue (* (Math|Vector|GetForwardVector _camera) (Variables|Default|GetOutlineRange))) (Utilities|Array|MakeArray "ObjectTypeQuery4") false 0 "None"))
      (if _returnvalue_2
        (if (== (.hitactor (Variables|Default|GetInteractable)) (.HitActor (Collision|BreakHitResult _outhit)))
          _
          (else
            (CallFunction|FOutlineTracing (.HitActor (Collision|BreakHitResult _outhit)) (.hitactor (Variables|Default|GetInteractable)))))
        (Variables|Default|SetInteractable _outhit)
        (else
          (Utilities|FlowControl|DoOnce false
            (:Completed
              (CallFunction|FOutlineStopTracing))))))))

(fn FOutlineTracing
  (params (New :type Actor%20Object%20Reference) (Previous :type Actor%20Object%20Reference))
  (Rendering|SetRenderCustomDepth (Actor|GetComponentbyClass New "/Script/Engine.PrimitiveComponent") true)
  (if (not (== Previous 0))
    (Rendering|SetRenderCustomDepth (Actor|GetComponentbyClass Previous "/Script/Engine.PrimitiveComponent") false)))

(fn FOutlineStopTracing
  (Utilities|FlowControl|Sequence
    (:then_0
      (if (not (== (.hitactor (Variables|Default|GetInteractable)) 0))
        (Rendering|SetRenderCustomDepth (Actor|GetComponentbyClass (.hitactor (Variables|Default|GetInteractable)) "/Script/Engine.PrimitiveComponent") false)))
    (:then_1
      (Variables|Default|SetInteractable ""))))