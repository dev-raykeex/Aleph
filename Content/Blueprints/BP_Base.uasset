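; BP_Base restores the saved UI style at startup and has the game instance build the matching HUD.
; BeginPlay copies UIStyle from the BP_SaveSettings slot into BP_Instance, or creates the save if missing, then calls CreateHUD for "Classic" or CreateAlternativeHUD otherwise.
; SaveSettings sets UIStyle on a loaded save without writing it back; it only writes a default save when none exists.
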(event EventBeginPlay
  (bind _returnvalue (Game|GetGameInstance))
  (bind _asbp_instance (Utilities|Casting|CastToBP_Instance _returnvalue))
  (bind _savec_1 (Variables|/Game/Blueprints/BP_Instance.BP_Instance_C|GetSaveC_1 _asbp_instance))
  (Utilities|FlowControl|Sequence
    (:then_0
      (bind _returnvalue_2 (SaveGame|DoesSaveGameExist _savec_1))
      (if _returnvalue_2
        (bind _returnvalue_3 (SaveGame|LoadGamefromSlot _savec_1))
        (bind _asbp_save_settings (Utilities|Casting|CastToBP_SaveSettings _returnvalue_3))
        (bind _asbp_instance_2 (Utilities|Casting|CastToBP_Instance (Game|GetGameInstance)))
        (Utilities|IsValid _asbp_instance_2
          (:Is%20Valid
            (Variables|/Script/Aleph.GInstance|SetUIStyle _asbp_instance_2 (Variables|/Script/Aleph.SaveSettings|GetUIStyle _asbp_save_settings))))
        (else
          (bind _returnvalue_4 (SaveGame|CreateSaveGameObject "/Game/Blueprints/Modules/BP_SaveSettings.BP_SaveSettings_C"))
          (SaveGame|SaveGametoSlot _returnvalue_4 _savec_1))))
    (:then_1
      (bind _asbp_instance_3 (Utilities|Casting|CastToBP_Instance (Game|GetGameInstance)))
      (if (Utilities|Enum|Equal(Enum) (Variables|/Script/Aleph.GInstance|GetUIStyle _asbp_instance_3) "Classic")
        (Default|CreateHUD _asbp_instance_3)
        (else
          (Default|CreateAlternativeHUD _asbp_instance_3))))))

(fn ConstructionScript)

(fn SaveSettings
  (params (UIStyle :type String))
  (bind _returnvalue (SaveGame|DoesSaveGameExist (Variables|Default|GetSaveC_1)))
  (if _returnvalue
    (bind _returnvalue_2 (SaveGame|LoadGamefromSlot (Variables|Default|GetSaveC_1)))
    (bind _asbp_save_settings (Utilities|Casting|CastToBP_SaveSettings _returnvalue_2))
    (Variables|/Script/Aleph.SaveSettings|SetUIStyle _asbp_save_settings UIStyle)
    (return)
    (else
      (bind _returnvalue_3 (SaveGame|CreateSaveGameObject "/Game/Blueprints/Modules/BP_SaveSettings.BP_SaveSettings_C"))
      (SaveGame|SaveGametoSlot _returnvalue_3 (Variables|Default|GetSaveC_1)))))