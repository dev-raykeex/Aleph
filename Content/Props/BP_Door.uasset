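; Interactive door prop that the player swings open and closed with the Interact input while near it.
; Box overlap events toggle input on the actor for player controller 0.
; Each press flips between playing and reversing a timeline that drives the Door component's yaw.
; When IsLocked is set, it instead sends a locked notification to the HUD held by the BP_Instance game instance.
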(event OnComponentBeginOverlap(Box)
  (params (OverlappedComponent :type Primitive%20Component%20Object%20Reference) (OtherActor :type Actor%20Object%20Reference) (OtherComp :type Primitive%20Component%20Object%20Reference) (OtherBodyIndex :type Integer) (bFromSweep :type Boolean) (SweepResult :type Hit%20Result%20Structure%20%28by%20ref%29))
  (Input|EnableInput (Game|GetPlayerController 0)))

(event OnComponentEndOverlap(Box)
  (params (OverlappedComponent :type Primitive%20Component%20Object%20Reference) (OtherActor :type Actor%20Object%20Reference) (OtherComp :type Primitive%20Component%20Object%20Reference) (OtherBodyIndex :type Integer))
  (Input|DisableInput (Game|GetPlayerController 0)))

(event Custom|Event%20OpenDoor
  ;[1 1 1] Custom Events
  (Utilities|FlowControl|FlipFlop
    (:A
      (bind _doorrotation (Timeline|OpenDoor Play)
        (:Update
          (Transformation|SetRelativeRotation (Variables|Default|GetDoor) (Math|Rotator|MakeRotator 0.0 0.0 _doorrotation) false false))))
    (:B
      (Timeline|OpenDoor Reverse))))

(event Input|ActionEvents|InputActionInteract
  (params (Key :type Key%20Structure))
  (:Pressed
    (if (Variables|Default|GetIsLocked)
      (CallFunction|AddNotification "This door is locked.")
      (else
        (CallFunction|EventOpenDoor)))))

(fn ConstructionScript)

(fn AddNotification
  (params (NotificationToShow :type Text))
  (bind _asbp_instance (Utilities|Casting|CastToBP_Instance (Game|GetGameInstance)))
  (Default|AddNotification (Variables|/Game/Blueprints/BP_Instance.BP_Instance_C|GetHeadsUpDisplay _asbp_instance) NotificationToShow "(R=0.102500,G=0.150000,B=0.000000,A=1.000000)" true 3.5))