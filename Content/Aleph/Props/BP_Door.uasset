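; BP_Door is an interactable door prop that swings open and closed, or shows a caption when locked.
; An overlap box enables input while overlapped, so Interact toggles a timeline that drives the door's yaw forward or in reverse.
; When locked, Interact instead sends a "door locked" closed caption through BP_Instance if captions are enabled, throttled by a DoOnce that resets after a random delay.
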(event OnComponentBeginOverlap(Box)
  (params (OverlappedComponent :type Primitive%20Component%20Object%20Reference) (OtherActor :type Actor%20Object%20Reference) (OtherComp :type Primitive%20Component%20Object%20Reference) (OtherBodyIndex :type Integer) (bFromSweep :type Boolean) (SweepResult :type Hit%20Result%20Structure%20%28by%20ref%29))
  (Input|EnableInput (Game|GetPlayerController 0)))

(event OnComponentEndOverlap(Box)
  (params (OverlappedComponent :type Primitive%20Component%20Object%20Reference) (OtherActor :type Actor%20Object%20Reference) (OtherComp :type Primitive%20Component%20Object%20Reference) (OtherBodyIndex :type Integer))
  (Input|DisableInput (Game|GetPlayerController 0)))

(event Custom|Event%20OpenDoor
  ;[1 1 1] Custom Events
  (Utilities|FlowControl|FlipFlop
    (:A
      (bind _doorrotation (Timeline|OpenDoor Play)
        (:Update
          (Transformation|SetRelativeRotation (Variables|Default|GetDoor) (Math|Rotator|MakeRotator 0.0 0.0 _doorrotation) false false))))
    (:B
      (Timeline|OpenDoor Reverse))))

(event Input|ActionEvents|InputActionInteract
  (params (Key :type Key%20Structure :default "None"))
  (:Pressed
    (if (Variables|Default|GetIsLocked)
      (Utilities|FlowControl|Sequence
        (:then_0
          (Utilities|FlowControl|DoOnce false :!label _label
            (:Completed
              (CallFunction|PlayCC))))
        (:then_1
          (Utilities|FlowControl|Delay (Math|Random|RandomFloatinRange 0.5 5.0))
          (goto _label Reset)))
      (else
        (CallFunction|EventOpenDoor)))))

(fn ConstructionScript)

(fn PlayCC
  (bind _returnvalue (Game|GetGameInstance))
  (bind _asbp_instance (Utilities|Casting|CastToBP_Instance _returnvalue))
  (if (Variables|/Script/Aleph.GInstance|GetEnableClosedCaptions _asbp_instance)
    (Default|SubtitlesHandler _asbp_instance 0 "" "*door locked*" 1.5 "(R=1.000000,G=0.375000,B=0.250000,A=1.000000)" true)))