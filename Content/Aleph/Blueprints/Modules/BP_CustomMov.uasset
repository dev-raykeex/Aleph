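; BP_CustomMov is a character movement module with an unfinished wall-run feature.
; Init caches the Character and default gravity, then starts a looping timer on an update event that is still empty, like Jump and Land.
; WRUpdate, not called here, line-traces for near-vertical walls while falling, stores the normal on player BP_Character and issues a zero-velocity launch.
; Helper graphs hold side-trace endpoint and normal-Z range math, shown unconnected.
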(event Custom|Init
  (params (Character :type Character%20Object%20Reference))
  (bind _output_get (Variables|Default|SetCharacter Character))
  (Variables|Default|SetDefaultGravity (Variables|/Script/Engine.CharacterMovementComponent|GetGravityScale (Variables|/Script/Engine.Character|GetCharacterMovement _output_get)))
  (Utilities|Time|SetTimerbyEvent (delegate Custom|EventWRUpdate) 0.02 true))

(event Custom|EventJump)

(event Custom|EventLand)

(event Custom|EventWRUpdate)

(fn WRUpdate
  (params (Start :type Vector) (End :type Vector) (WR_Direction :type Float%20%28single-precision%29))
  (bind _outhit (Collision|LineTraceByChannel Start End "TraceTypeQuery1" false 0 "None"))
  (if (.bblockinghit _outhit)
    (if (and (AI|Components|NavMovement|IsFalling (Variables|/Script/Engine.Character|GetCharacterMovement (Variables|Default|GetCharacter))) (.Return (Utilities|WRValidWallCheck (.normal _outhit))))
      (bind _asbp_character (Utilities|Casting|CastToBP_Character (Game|GetPlayerCharacter 0)))
      (Utilities|IsValid _asbp_character
        (:Is%20Valid
          (Variables|/Script/Aleph.PCharacter|SetWR_Normal _asbp_character (.InVec2 (Utilities|WRValidWallCheck (.normal _outhit))))
          (Character|LaunchCharacter (Variables|Default|GetCharacter) "0, 0, 0" false false))))))