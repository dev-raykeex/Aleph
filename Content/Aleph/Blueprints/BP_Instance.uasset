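; Game instance for Aleph that persists player settings and provides shared UI helpers.
; Init reads UI style and mouse sensitivity from the SaveC1 slot via BP_SaveSettings, and Shutdown writes them back.
; Separate functions create and display the NoUI, Aleph, Alternative and Classic HUD widgets.
; Notification and subtitle handlers broadcast messages to every NotificationTray or W_SubGrid widget found, with subtitles gated by EnableSubtitles.
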(event EventInit
  (Utilities|FlowControl|Sequence
    (:then_0
      (bind _returnvalue (SaveGame|DoesSaveGameExist (Variables|Default|GetSaveC_1)))
      (if _returnvalue
        (bind _returnvalue_2 (SaveGame|LoadGamefromSlot (Variables|Default|GetSaveC_1)))
        (bind _asbp_save_settings (Utilities|Casting|CastToBP_SaveSettings _returnvalue_2))
        (Variables|Default|SetUIStyle (Variables|/Script/Aleph.SaveSettings|GetUIStyle_SValue _asbp_save_settings))))
    (:then_1
      (bind _mouse_sensitivity_svalue (CallFunction|LoadSettings (Variables|Default|GetSaveC_1)))
      (Variables|Default|SetMouseSensitivity _mouse_sensitivity_svalue))))

(event EventShutdown
  (CallFunction|SaveSettings (Variables|Default|GetSaveC_1)))

(fn CreateNoUI
  (bind _returnvalue (UserInterface|CreateWidget "/Game/Aleph/Widgets/NoUI.NoUI_C" (Game|GetPlayerController 0)))
  (bind _output_get (Variables|Default|SetHUD_00 _returnvalue))
  (Utilities|IsValid _output_get
    (:Is%20Valid
      (UserInterface|Viewport|AddtoViewport _output_get 0))))

(fn CreateAleph
  (bind _returnvalue (UserInterface|CreateWidget "/Game/Aleph/Widgets/Aleph.Aleph_C" (Game|GetPlayerController 0)))
  (bind _output_get (Variables|Default|SetHUD_01 _returnvalue))
  (Utilities|IsValid _output_get
    (:Is%20Valid
      (UserInterface|Viewport|AddtoViewport _output_get 0))))

(fn CreateAlternative
  (bind _returnvalue (UserInterface|CreateWidget "/Game/Aleph/Widgets/Alternative.Alternative_C" (Game|GetPlayerController 0)))
  (bind _output_get (Variables|Default|SetHUD_02 _returnvalue))
  (Utilities|IsValid _output_get
    (:Is%20Valid
      (UserInterface|Viewport|AddtoViewport _output_get 0))))

(fn CreateClassic
  (bind _returnvalue (UserInterface|CreateWidget "/Game/Aleph/Widgets/Classic.Classic_C" (Game|GetPlayerController 0)))
  (bind _output_get (Variables|Default|SetHUD_03 _returnvalue))
  (UserInterface|Viewport|AddtoViewport _output_get 0))

(fn LoadSettings
  (params (SlotName :type String))
  (bind _returnvalue (SaveGame|DoesSaveGameExist SlotName))
  (if _returnvalue
    (bind _returnvalue_2 (SaveGame|LoadGamefromSlot SlotName))
    (bind _asbp_save_settings (Utilities|Casting|CastToBP_SaveSettings _returnvalue_2)
      (:CastFailed
        (bind _returnvalue_3 (SaveGame|CreateSaveGameObject "/Game/Aleph/Blueprints/Modules/BP_SaveSettings.BP_SaveSettings_C"))
        (bind _output_get (Variables|Default|SetSettings _returnvalue_3))
        (bind _returnvalue_4 (SaveGame|SaveGametoSlot _output_get SlotName))
        (if _returnvalue_4
          _
          (else
            (Development|PrintString "ERROR: The game failed to save the Settings in the loading function.")))
        (return (Variables|Default|GetSettings) (Variables|/Script/Aleph.SaveSettings|GetMouseSensitivity_SValue _asbp_save_settings))))
    (else
      (bind _returnvalue_5 (SaveGame|CreateSaveGameObject "/Game/Aleph/Blueprints/Modules/BP_SaveSettings.BP_SaveSettings_C"))
      (Variables|Default|SetSettings _returnvalue_5))))

(fn SaveSettings
  (params (SlotName :type String))
  (bind _returnvalue (SaveGame|DoesSaveGameExist SlotName))
  (if _returnvalue
    (bind _returnvalue_2 (SaveGame|LoadGamefromSlot (Variables|Default|GetSaveC_1)))
    (bind _asbp_save_settings (Utilities|Casting|CastToBP_SaveSettings _returnvalue_2))
    (Variables|/Script/Aleph.SaveSettings|SetUIStyle_SValue _asbp_save_settings (Variables|Default|GetUIStyle))
    (Variables|/Script/Aleph.SaveSettings|SetMouseSensitivity_SValue _asbp_save_settings (Variables|Default|GetMouseSensitivity))
    (SaveGame|SaveGametoSlot _asbp_save_settings (Variables|Default|GetSaveC_1))
    (else
      (bind _returnvalue_3 (SaveGame|CreateSaveGameObject "/Game/Aleph/Blueprints/Modules/BP_SaveSettings.BP_SaveSettings_C"))
      (Variables|/Script/Aleph.SaveSettings|SetUIStyle_SValue _returnvalue_3 (Variables|Default|GetUIStyle))
      (Variables|/Script/Aleph.SaveSettings|SetMouseSensitivity_SValue _returnvalue_3 (Variables|Default|GetMouseSensitivity))
      (SaveGame|SaveGametoSlot _returnvalue_3 (Variables|Default|GetSaveC_1)))))

(fn NotificationHandler
  (params (Notification :type Text) (NotificationColor :type Linear%20Color%20Structure :default "(R=0.102500,G=0.150000,B=0.000000,A=0.700000)") (NotificationRemoval :type Boolean) (NotificationRemovalTime :type Float%20%28single-precision%29))
  (bind _foundwidgets (Widget|GetAllWidgetsOfClass "/Game/Aleph/Widgets/Elements/Notifications/NotificationTray.NotificationTray_C" false))
  (for _array_element _foundwidgets
    (Utilities|IsValid _array_element
      (:Is%20Valid
        (Default|SetNotification _array_element Notification NotificationColor NotificationRemoval NotificationRemovalTime)))))

(fn SubtitlesHandler
  (params (Audio :type Sound%20Base%20Object%20Reference) (Character :type Text) (Subtitles :type Text) (ScreenTime :type Float%20%28single-precision%29) (Color :type Linear%20Color%20Structure :default "(R=1.000000,G=1.000000,B=1.000000,A=1.000000)"))
  (if (Variables|Default|GetEnableSubtitles)
    (bind _foundwidgets (Widget|GetAllWidgetsOfClass "/Game/Aleph/Widgets/Elements/Subtitles/W_SubGrid.W_SubGrid_C" false))
    (for _array_element _foundwidgets
      (Utilities|IsValid _array_element
        (:Is%20Valid
          (Class|BPISubtitles|PlaySubtitles(Message) _array_element Audio Character Subtitles ScreenTime Color))))))