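; BP_Aleph is a game mode that handles player logins and broadcasts chat messages.
; On PostLogin it records each BP_Controller in OnlinePlayers, then spawns and possesses a BP_Character named after the player.
; Spawn points come from FindPlayerStart, using the player's index in that array as the start name.
; SendGlobalMessages relays a sender and message to every tracked controller's chat.
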(event Custom|SendGlobalMessages
  (params (Sender :type String) (Message :type String))
  (for _array_element (Variables|Default|GetOnlinePlayers)
    (Default|AddMessagetoChat _array_element Sender Message)))

(event Custom|OnLogin
  (params (NewPlayer :type Player%20Controller%20Object%20Reference))
  (bind _asbp_controller (Utilities|Casting|CastToBP_Controller NewPlayer))
  (Utilities|Array|Add (Variables|Default|GetOnlinePlayers) _asbp_controller)
  (bind _returnvalue (Game|SpawnActorfromClass "/Game/Aleph/Blueprints/BP_Character.BP_Character_C" (Transformation|GetActorTransform (Class|GameModeBase|FindPlayerStart NewPlayer (Utilities|String|ToString(Integer) (- (Utilities|Array|Length (Variables|Default|GetOnlinePlayers)) 1)))) "Undefined" 0 (PlayerState|GetPlayerName (Variables|/Script/Engine.Controller|GetPlayerState NewPlayer)) 0))
  (Pawn|Possess _asbp_controller _returnvalue))

(event EventPostLogin
  (params (NewPlayer :type Player%20Controller%20Object%20Reference))
  (CallFunction|OnLogin NewPlayer))

(fn ConstructionScript)