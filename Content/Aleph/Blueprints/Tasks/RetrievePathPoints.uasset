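; Behavior tree task that feeds a Drone the next point of its patrol path.
; It reads the path index from the blackboard, converts that local path point to world space through the patrol path actor's transform, and writes it back as a vector.
; It also sets the patrolling flag, failing and clearing it when the drone has no valid path.
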(event EventReceiveExecuteAI
  (params (OwnerController :type AI%20Controller%20Object%20Reference) (ControlledPawn :type Pawn%20Object%20Reference))
  (bind _bb_isaipatrolling (Variables|Default|GetBB_IsAIPatrolling))
  (bind _asdrone (Utilities|Casting|CastToDrone ControlledPawn))
  (bind _dronepatrolpath (Variables|/Game/Aleph/Blueprints/AI/Drone/Drone.Drone_C|GetDronePatrolPath _asdrone)
    (:then
      (Class|BTFunctionLibrary|SetBlackboardValueasBool _bb_isaipatrolling true)
      (AI|BehaviorTree|SetBlackboardValueasVector (Variables|Default|GetBB_PathV) (Math|Transform|TransformLocation (Transformation|GetActorTransform _dronepatrolpath) (Utilities|Array|Get(acopy) (Variables|/Game/Aleph/Blueprints/AI/BP_PatrolPath.BP_PatrolPath_C|GetPathPoints _dronepatrolpath) (Class|BTFunctionLibrary|GetBlackboardValueasInt (Variables|Default|GetBB_PathIndex)))))
      (AI|BehaviorTree|FinishExecute true))
    (:else
      (Class|BTFunctionLibrary|SetBlackboardValueasBool _bb_isaipatrolling false)
      (AI|BehaviorTree|FinishExecute false))))