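; BP_Base is an actor that persists player settings to a save game when play ends.
; On EndPlay it reads UIStyle from the player's BP_HUD and passes it to SaveSettings.
; SaveSettings loads or creates a BP_SaveSettings object in the SaveC1 slot, writes UI style and mouse sensitivity, then saves it.
; EndPlay passes zero for sensitivity, so each such save overwrites any stored sensitivity.
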(event EventEndPlay
  (params (EndPlayReason :type EEndPlayReason%20Enum :default "Destroyed"))
  (bind _asbp_hud (Utilities|Casting|CastToBP_HUD (HUD|GetHUD (Game|GetPlayerController 0))))
  (CallFunction|SaveSettings (Variables|/Script/Aleph.MainHUD|GetUIStyle _asbp_hud) 0.0))

(fn ConstructionScript)

(fn SaveSettings
  (params (UIStyle :type String) (Mouse%20Sensitivity%20SValue :type Float%20%28single-precision%29))
  (bind _returnvalue (SaveGame|DoesSaveGameExist (Variables|Default|GetSaveC_1)))
  (if _returnvalue
    (bind _returnvalue_2 (SaveGame|LoadGamefromSlot (Variables|Default|GetSaveC_1)))
    (bind _asbp_save_settings (Utilities|Casting|CastToBP_SaveSettings _returnvalue_2))
    (Variables|/Script/Aleph.SaveSettings|SetUIStyle _asbp_save_settings UIStyle)
    (Variables|/Script/Aleph.SaveSettings|SetSensitivity _asbp_save_settings Mouse%20Sensitivity%20SValue)
    (SaveGame|SaveGametoSlot _asbp_save_settings (Variables|Default|GetSaveC_1))
    (else
      (bind _returnvalue_3 (SaveGame|CreateSaveGameObject "/Game/Aleph/Blueprints/Modules/BP_SaveSettings.BP_SaveSettings_C"))
      (Variables|/Script/Aleph.SaveSettings|SetUIStyle _returnvalue_3 UIStyle)
      (Variables|/Script/Aleph.SaveSettings|SetSensitivity _returnvalue_3 Mouse%20Sensitivity%20SValue)
      (SaveGame|SaveGametoSlot _returnvalue_3 (Variables|Default|GetSaveC_1)))))