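; BP_Button is a UI button that keeps mouse hover and keyboard focus in sync for menu highlighting.
; Begin starts a looping timer that polls CheckFocus several times a second instead of relying on hover or focus events.
; A hovered button takes keyboard focus and shows the mouse style; otherwise its style switches between selected and not selected according to keyboard focus.
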(fn Begin
  (Utilities|Time|SetTimerbyFunctionName 0 "CheckFocus" 0.1 true))

(fn CheckFocus
  (if (Widget|IsHovered)
    (Widget|SetKeyboardFocus)
    (Class|Button|SetStyle (Variables|Default|GetMouseS))
    (else
      (Class|Button|SetStyle (select (Class|Widget|HasKeyboardFocus) (Variables|Default|GetSelected) (Variables|Default|GetNotSelected))))))